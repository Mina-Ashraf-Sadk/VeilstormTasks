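; Game mode for Map1 that admits players up to a map capacity, splits them into two teams and handles their deaths.
; On login it tags the controller T1 or T2 by team size, then spawns and possesses a character at a free team spawn point, consuming that point's Free tag.
; KillPlayer destroys the pawn, notifies listeners and spawns a death drop.
; Kicking players from a full game is marked as not working.
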(event Custom|KillPlayer
  (params (PlayerController :type Controller%20Object%20Reference))
  (CallFunction|DestroyPlayer PlayerController))

(event EventPostLogin
  (params (NewPlayer :type Player%20Controller%20Object%20Reference))
  (CallFunction|HandleNewPlayer NewPlayer))

(fn ConstructionScript)

(fn HandleNewPlayer
  (params (NewPlayer :type Player%20Controller%20Object%20Reference%20%28by%20ref%29))
  (if (< (Utilities|Array|Length (Variables|Game|GetPlayers)) (Variables|Default|GetMapCapacity))
    ;[1 1 1] Spawn Player and add to players list
    (CallFunction|AutoAssigntoTeam NewPlayer)
    (CallFunction|SpawnPlayer NewPlayer)
    (Utilities|Array|AddUnique (Variables|Game|GetPlayers) NewPlayer)
    (else
      ;[1 1 1] should kick player but currently not working
      (CallFunction|KickPlayer NewPlayer))))

(fn KickPlayer
  (params (Player :type Player%20Controller%20Object%20Reference%20%28by%20ref%29))
  (bind _aspc_veilstorm_tasks_controller (Utilities|Casting|CastToPC_VeilstormTasksController Player))
  (Class|AdvancedSessionsLibrary|KickPlayer _aspc_veilstorm_tasks_controller "Game Is Full"))

(fn SpawnPlayer
  (params (PlayerToSpawn :type Controller%20Object%20Reference))
  (bind _availablespawntransform (CallFunction|FetchSpawnLocation PlayerToSpawn))
  (bind _returnvalue (Game|SpawnActorfromClass "/Game/VeilstormTasks/Characters/BP_ThirdPersonCharacter.BP_ThirdPersonCharacter_C" _availablespawntransform "Undefined" "MultiplyWithRoot" PlayerToSpawn 0))
  (Pawn|Possess PlayerToSpawn _returnvalue)
  (Class|BPIDeathInterface|OnSpawn(Message) PlayerToSpawn))

(fn AutoAssigntoTeam
  (params (PlayerController :type Player%20Controller%20Object%20Reference))
  (bind _tags (Variables|/Script/Engine.Actor|GetTags PlayerController))
  (bind (_team1players _team2players) (|CalculatesTheNumberOfPlayersInEachTeam)
    (:Completed
      (if (<= _team1players _team2players)
        (Utilities|Array|Add _tags "T1")
        (else
          (Utilities|Array|Add _tags "T2"))))))

(fn FetchSpawnLocation
  (params (PlayerController :type Controller%20Object%20Reference))
  (if (Actor|ActorHasTag PlayerController "T1")
    (LocalVariables|SetSearchTeam "NewEnumerator1")
    (else
      (LocalVariables|SetSearchTeam "NewEnumerator0")))
  (if (> (Utilities|Array|Length (Variables|Default|GetSpawnLocations)) 0) :!label _label
    (for _array_element (Variables|Default|GetSpawnLocations)
      (if (and (Utilities|Enum|Equal(Enum) (Variables|/Game/VeilstormTasks/Blueprints/LevelActors/BP_SpawnPoint.BP_SpawnPoint_C|GetTeam _array_element) (LocalVariables|GetSearchTeam)) (Utilities|Array|ContainsItem (Variables|/Script/Engine.Actor|GetTags _array_element) "Free"))
        (LocalVariables|SetSpawnPoint _array_element)))
    (if (Utilities|IsValid (LocalVariables|GetSpawnPoint))
      (Utilities|Array|RemoveItem (Variables|/Script/Engine.Actor|GetTags (LocalVariables|GetSpawnPoint)) "Free")
      (return (Transformation|GetActorTransform (LocalVariables|GetSpawnPoint)))
      (else
        (Development|PrintString "No Available Spawn Points Found Spawn At 000" true true "(R=0.000000,G=0.660000,B=1.000000,A=1.000000)" 1e+01)
        (return (Math|Transform|MakeTransform "0, 0, 0" "0, 0, 0" "1.000000,1.000000,1.000000"))))
    (else
      (Development|PrintString "NoSessionsFoundSearchingAgain(This will cause an infinit loop if no spawn points were on the map)")
      (Utilities|UpdateSpawnLocations)
      (goto _label))))

(fn DestroyPlayer
  (params (Player :type Controller%20Object%20Reference))
  (LocalVariables|SetLastLoc (Transformation|GetActorLocation (Pawn|GetControlledPawn Player)))
  ;[1 1 1] Destroy the player pawn and call the death delegate
  (Actor|DestroyActor (Pawn|GetControlledPawn Player))
  (Class|BPIDeathInterface|OnDeath(Message) Player 5)
  (Default|CallOnPlayerDeath)
  ;[1 1 1] Spawn the death drop (health and ammo)
  (Game|SpawnActorfromClass "/Game/VeilstormTasks/Blueprints/LevelActors/DeathDrop.DeathDrop_C" (Math|Conversions|ToTransform(Vector) (LocalVariables|GetLastLoc)) "Undefined" "MultiplyWithRoot" 0 0))