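; Matchmaking menu controller that shows the EOS main menu widget on BeginPlay with mouse cursor and UI-only input.
; It hands start and cancel events to the widget, which toggle the player's online ready state when logged in.
; Otherwise both trigger AutoLogin and print the result, without retrying the ready change.
; Start also fills a hard-coded 1v1 host configuration, though nothing here reads it.
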(event Custom|LoginUser
  (bind (_bwassuccessful _userid _error) (|AutoLogin (Subsystems|GetOnlineIdentitySubsystem))
    (:OnCallFailed
      (Development|PrintString (Utilities|String|Append "Login Failed Error:  " _error)))
    (:OnLoginComplete
      (Development|PrintString (Utilities|String|Append "  User Logged in   :" (Utilities|String|ToString(Integer) _userid))))))

(event Custom|StartMatchmaking_Event
  (Variables|Default|SetHostConfiguration (Utilities|Struct|MakeMatchmakerHostConfiguration "test" "1v1" true 10 5 false "" false "/Game/VeilstormTasks/Maps/Map2.Map2" 0 "9990"))
  (if (Class|KismetSystemLibrary|IsLoggedin (Game|GetPlayerController 0))
    (Class|Matchmaker|SetReadyState (Utilities|Struct|MakeUniqueNetIdRepl) true)
    (Development|PrintString "Player Ready")
    (else
      (Development|PrintString "Not Logged in")
      (CallFunction|LoginUser))))

(event Custom|CancelMatchmaking_Event
  (if (Class|KismetSystemLibrary|IsLoggedin (Game|GetPlayerController 0))
    (Class|Matchmaker|SetReadyState (Utilities|Struct|MakeUniqueNetIdRepl) false)
    (Development|PrintString "Player Unready")
    (else
      (CallFunction|LoginUser))))

(event EventBeginPlay
  (bind _returnvalue (Game|GetPlayerController 0))
  (Variables|/Script/Engine.PlayerController|SetbShowMouseCursor _returnvalue true)
  (bind _returnvalue_2 (UserInterface|CreateWidget "/Game/VeilstormTasks/UI/WBP_EOSMainMenu.WBP_EOSMainMenu_C" _returnvalue))
  (bind _output_get (Variables|Default|SetMenuUI _returnvalue_2))
  (UserInterface|Viewport|AddtoViewport _output_get 0)
  (Input|SetInputModeUIOnly (Game|GetPlayerController 0) 0 "DoNotLock" false)
  (EventDispatchers|AssignStartMatchmaking (Variables|Default|GetMenuUI) (delegate Custom|StartMatchmaking_Event))
  (EventDispatchers|AssignCancelMatchmaking (Variables|Default|GetMenuUI) (delegate Custom|CancelMatchmaking_Event)))

(fn ConstructionScript)