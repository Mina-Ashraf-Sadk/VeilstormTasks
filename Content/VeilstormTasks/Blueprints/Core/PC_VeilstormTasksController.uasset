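; Player controller for VeilstormTasks that manages the HUD, scoreboard, death countdown and respawn requests.
; OnSpawn creates the HUD once, holding Tab shows a lazily created scoreboard, and LeaveSession delegates to the advanced game instance.
; OnDeath starts a looping one-second timer that counts DeathTimer down, then enables respawn.
; The respawn input triggers Respawn, commented as server-side, which checks that state before asking GM_Map1 to spawn the player.
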(event Custom|LeaveSession
  ;[1 0 0] Leave Session
  (bind _asgi_advanced_game_instance (Utilities|Casting|CastToGI_AdvancedGameInstance (Game|GetGameInstance)))
  (Default|LeaveCurrentSession _asgi_advanced_game_instance))

(event Custom|Respawn
  ;[0 0.08183 1] Server Respawn
  (if (and (<= (Variables|Default|GetDeathTimer) 0.0) (Variables|Default|GetbCanRespawn))
    (bind _asgm_map_1 (Utilities|Casting|CastToGM_Map1 (Game|GetGameMode)))
    (Default|SpawnPlayer _asgm_map_1 self)
    (Variables|Default|SetbCanRespawn false)))

(event Custom|DisplayHUD
  ;[1 0 0] Display The HUD
  (Utilities|IsValid (Variables|Default|GetHUD)
    (:Is%20Not%20Valid
      (bind _returnvalue (UserInterface|CreateWidget "/Game/VeilstormTasks/UI/WBP_HUD.WBP_HUD_C" self))
      (bind _output_get (Variables|Default|SetHUD _returnvalue))
      (UserInterface|Viewport|AddtoViewport _output_get 0))))

(event Input|EnhancedActionEvents|EnhancedInputActionIA_Respawn
  (params (ActionValue :type Boolean) (ElapsedSeconds :type Float%20%28double-precision%29) (TriggeredSeconds :type Float%20%28double-precision%29) (InputAction :type Input%20Action%20Object%20Reference :default "/Game/VeilstormTasks/Blueprints/Input/Actions/IA_Respawn.IA_Respawn"))
  ;[1 0 0] Cleint Request to Respawn
  (:Started
    (CallFunction|Respawn)))

(event EventOnDeath
  (params (DeathTime :type Integer))
  ;[1 0 0] OnDeathEvent that starts the death timer ......how to make the death timer a constant ?
  (Variables|Default|SetDeathTimer DeathTime)
  (Variables|Default|SetbCanRespawn false)
  (Utilities|Time|SetTimerbyFunctionName 0 "ReduceDeathTimer" 1.0 true))

(event EventOnSpawn
  ;[1 0 0] Display The HUD
  (CallFunction|DisplayHUD))

(event Input|KeyboardEvents|Tab
  (params (Key :type Key%20Structure :default "None"))
  (:Pressed
    (Utilities|IsValid (Variables|Default|GetScoreBoard)
      (:Is%20Valid
        (Widget|SetVisibility (Variables|Default|GetScoreBoard) "Visible"))
      (:Is%20Not%20Valid
        (bind _returnvalue (UserInterface|CreateWidget "/Game/VeilstormTasks/UI/WBP_ScoreBoard.WBP_ScoreBoard_C"))
        (bind _output_get (Variables|Default|SetScoreBoard _returnvalue))
        (UserInterface|Viewport|AddtoViewport _output_get 0))))
  (:Released
    (Widget|SetVisibility (Variables|Default|GetScoreBoard) "Hidden")))

(fn ConstructionScript)

(fn ReduceDeathTimer
  (bind _result (Math|Integer|DecrementInt (Variables|Default|GetDeathTimer))
    (:%20%20
      (if (<= _result 0)
        (Variables|Default|SetDeathTimer 0)
        (Utilities|Time|ClearTimerbyFunctionName 0 "ReduceDeathTimer")
        (Variables|Default|SetbCanRespawn true)))))

(fn OnRepDeathTimer)