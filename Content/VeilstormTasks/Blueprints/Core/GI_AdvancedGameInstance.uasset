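; Game instance that handles multiplayer matchmaking through Advanced Sessions nodes, along with leaving sessions and accepting invites.
; JoinBattle searches sessions, keeps those matching the selected map with free slots, then tries to join a low-ping one that is not banned.
; Failed joins ban that session ID and retry from the earlier search results.
; When no suitable session exists, it creates one tagged with the map and opens that level as a listen server.
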(event Custom|JoinBattle
  (params (CurrentLevel :type Name) (ServerCapacity :type Integer))
  ;[1 1 1] Register the map and it's capacity and search for any sessions if none found create your own
  (Variables|SessionSettings|SetServerCapacity ServerCapacity)
  (Variables|SessionSettings|SetSelectedLevel CurrentLevel)
  (bind _results (|FindSessionsAdvanced (Game|GetPlayerController 0) 10000 false "AllServers" 0 false false false false)
    (:OnSuccess
      _)
    (:OnFailure
      _))
  (if (Utilities|Array|IsEmpty _results)
    (Utilities|CreateNewSession)
    (else
      (Utilities|SearchAvailableSessions _results
        (:Connected
          ;[1 1 1] if connected succussfully Print The joined session name
          (Development|PrintString (Utilities|String|Append "Connected To Session " (Class|FindSessionsCallbackProxy|GetServerName (Variables|Properties|GetFoundSession)))))
        (:Failed%20To%20connect
          ;[1 1 1] if failed to connect to the found session ban it and  Search Again
          (Utilities|Array|AddUnique (Variables|SearchResult|GetBannedSessions) (Class|AdvancedSessionsLibrary|GetSessionIDasString (Variables|Properties|GetFoundSession)))
          (|DestroySession (Game|GetPlayerController 0)
            (:OnSuccess
              (CallFunction|TryAgain)
              (Development|PrintString "Session found but connection failed"))
            (:OnFailure
              (CallFunction|JoinBattle (Variables|SessionSettings|GetSelectedLevel) (Variables|SessionSettings|GetServerCapacity))
              (Development|PrintString "Session found but connection failed"))))
        (:None%20Found
          ;[1 1 1] if no suitable session found create your own
          (Development|PrintString "Sessions Found But no Suitable one found")
          (Utilities|CreateNewSession))))))

(event Custom|LeaveCurrentSession
  ;[1 1 1] leave session
  (|DestroySession (Game|GetPlayerController 0)
    (:OnSuccess
      (Game|OpenLevel(byObjectReference) "/Game/VeilstormTasks/Maps/MainMenu.MainMenu"))))

(event Custom|CancelSearch
  ;[1 1 1] Cancel Search
  (|CancelFindSessions (Game|GetPlayerController 0)))

(event Custom|TryAgain
  (Utilities|SearchAvailableSessions (stale Custom|JoinBattle _results)
    (:Connected
      ;[1 1 1] if connected succussfully Print The joined session name
      (Development|PrintString (Utilities|String|Append "Connected To Session " (Class|FindSessionsCallbackProxy|GetServerName (Variables|Properties|GetFoundSession)))))
    (:Failed%20To%20connect
      ;[1 1 1] if failed to connect to the found session ban it and  Search Again
      (Utilities|Array|AddUnique (Variables|SearchResult|GetBannedSessions) (Class|AdvancedSessionsLibrary|GetSessionIDasString (Variables|Properties|GetFoundSession)))
      (|DestroySession (Game|GetPlayerController 0)
        (:OnSuccess
          (CallFunction|TryAgain)
          (Development|PrintString "Session found but connection failed"))
        (:OnFailure
          (CallFunction|JoinBattle (Variables|SessionSettings|GetSelectedLevel) (Variables|SessionSettings|GetServerCapacity))
          (Development|PrintString "Session found but connection failed"))))
    (:None%20Found
      ;[1 1 1] if no suitable session found create your own
      (Development|PrintString "Sessions Found But no Suitable one found")
      (Utilities|CreateNewSession))))

(event EventOnSessionInviteAccepted
  (params (LocalPlayerNum :type Integer) (PersonInvited :type BP%20Unique%20Net%20Id%20Structure) (SessionToJoin :type Blueprint%20Session%20Result%20Structure%20%28by%20ref%29))
  (|JoinSession (Game|GetPlayerController 0) SessionToJoin))