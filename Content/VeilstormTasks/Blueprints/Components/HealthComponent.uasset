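; Health component that applies damage to its owning actor, blocks friendly fire and handles player death in a team-based match.
; It binds to the owner's any-damage event and passes both instigator controllers to a server-named event that reduces health.
; A macro compares T1/T2 controller tags to reject teammate hits.
; Valid hits record damage on PlayerState; lethal ones also record kill and death, then call GM_Map1 to kill the player.
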(event Custom|OnTakeAnyDamage_Event
  (params (DamagedActor :type Actor%20Object%20Reference) (Damage :type Float%20%28single-precision%29) (DamageType :type Damage%20Type%20Object%20Reference) (InstigatedBy :type Controller%20Object%20Reference) (DamageCauser :type Actor%20Object%20Reference))
  (CallFunction|ServerReduceHP (Pawn|GetController (Variables|/Script/Engine.Actor|GetInstigator DamagedActor)) Damage (Pawn|GetController (Variables|/Script/Engine.Actor|GetInstigator DamageCauser))))

(event Custom|Server_ReduceHP
  (params (DamagedPlayer :type Controller%20Object%20Reference) (Damage :type Float%20%28double-precision%29) (DamageCauser :type Controller%20Object%20Reference))
  (CallFunction|ReduceHealth DamagedPlayer Damage DamageCauser))

(event EventBeginPlay
  (EventDispatchers|AssignOnTakeAnyDamage (Components|GetOwner) (delegate Custom|OnTakeAnyDamage_Event)))

(fn ReduceHealth
  (params (DamagedPlayer :type Controller%20Object%20Reference) (Damage :type Float%20%28double-precision%29) (DamageCauser :type Controller%20Object%20Reference))
  (Utilities|CheckFriendlyFire DamagedPlayer DamageCauser
    (:Valid
      (Class|BPIScoreBoardInterface|RecordDamage(Message) (Variables|/Script/Engine.Controller|GetPlayerState DamageCauser) Damage)
      (bind _output_get (LocalVariables|SetCalculatedDamage (- (Variables|Default|GetHealth) Damage)))
      (if (> _output_get 0.0)
        (bind _output_get_2 (Variables|Default|SetHealth (LocalVariables|GetCalculatedDamage)))
        (Development|PrintString (Utilities|String|ToString(Float) _output_get_2))
        (else
          (Class|BPIScoreBoardInterface|GainDeath(Message) (Variables|/Script/Engine.Controller|GetPlayerState DamagedPlayer))
          (Class|BPIScoreBoardInterface|GainKill(Message) (Variables|/Script/Engine.Controller|GetPlayerState DamageCauser))
          (bind _asgm_map_1 (Utilities|Casting|CastToGM_Map1 (Game|GetGameMode)))
          (Default|KillPlayer _asgm_map_1 DamagedPlayer))))
    (:NotValid
      (Development|PrintString "FriendlyFireNotAllowed!! If you hate your teammates just insult them in chat"))))