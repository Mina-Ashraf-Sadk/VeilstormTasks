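; Multiplayer weapon component for Characters that handles equipping, aiming, shooting and reloading.
; Weapon data assets drive the spawned, socket-attached weapon, fire mode and ammo, and the AnimBP receives updates through a weapon interface.
; The client traces from camera center, then the server re-traces from the client-sent muzzle to apply bone-based damage and reduce the magazine.
; Server RPCs, multicasts and RepNotifies replicate aim rotation and animations.
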(event Custom|ServerReduceMag
  (params (Target :type DABP%20Weapon%20Info%20Object%20Reference))
  (CallFunction|ReduceMag))

(event Custom|Server_Reload
  (params (InSkeletalMeshComponent :type Skeletal%20Mesh%20Component%20Object%20Reference) (MontageToPlay :type Anim%20Montage%20Object%20Reference))
  (Variables|Default|SetbReloading true)
  (CallFunction|MCReloadAnim InSkeletalMeshComponent MontageToPlay))

(event Custom|Server_RepAimRot
  (params (AimRotation :type Rotator))
  (Variables|Default|SetAimRotation AimRotation))

(event Custom|MC_SpawnEffect
  (params (EmitterTemplate :type Particle%20System%20Object%20Reference) (Location :type Vector) (Rotation :type Rotator))
  (Effects|SpawnEmitteratLocation EmitterTemplate Location Rotation))

(event Custom|Server_SpawnEffect
  (params (EmitterTemplate :type Particle%20System%20Object%20Reference) (Location :type Vector) (Rotation :type Rotator))
  (CallFunction|MCSpawnEffect EmitterTemplate Location Rotation))

(event Custom|MC_PlayAnim
  (params (NewAnimToPlay :type Animation%20Asset%20Object%20Reference) (bLooping :type Boolean))
  ;[1 1 1] MultiCasting the animation to everyone but the client cause they already played it
  (if (not (Pawn|IsLocallyControlled (Variables|CharacterReferances|GetCharacter)))
    (Components|Animation|PlayAnimation (Variables|/Game/VeilstormTasks/Blueprints/Weapons/BP_MasterWeapon.BP_MasterWeapon_C|GetSkeletalMesh (Variables|WeaponData|GetCurrentWeapon)) NewAnimToPlay bLooping)))

(event Custom|Server_PlayAnim
  (params (NewAnimToPlay :type Animation%20Asset%20Object%20Reference) (bLooping :type Boolean))
  (CallFunction|MCPlayAnim NewAnimToPlay bLooping))

(event Custom|Server_ShootLineTrace
  (params (MuzzleLocation :type Vector) (CameraCenterEndLine :type Vector) (DamageCauser :type Actor%20Object%20Reference) (Target :type DABP%20Weapon%20Info%20Object%20Reference))
  (if (CallFunction|CanShoot)
    (CallFunction|ServerDamageCalc MuzzleLocation CameraCenterEndLine DamageCauser)
    (CallFunction|ReduceMag)))

(event Custom|MC_ReloadAnim
  (params (InSkeletalMeshComponent :type Skeletal%20Mesh%20Component%20Object%20Reference) (MontageToPlay :type Anim%20Montage%20Object%20Reference))
  (Animation|Montage|PlayMontage InSkeletalMeshComponent MontageToPlay
    (:OnBlendOut
      _)
    (:OnInterrupted
      _))
  (Variables|Default|SetbReloading false)
  (CallFunction|ReloadCalc))

(event Custom|SR_Aiming
  (params (bAiming :type Boolean))
  (Variables|Default|SetbAiming bAiming))

(event Input|EnhancedActionEvents|EnhancedInputActionIA_Aim
  (params (ActionValue :type Boolean) (ElapsedSeconds :type Float%20%28double-precision%29) (TriggeredSeconds :type Float%20%28double-precision%29) (InputAction :type Input%20Action%20Object%20Reference :default "/Game/VeilstormTasks/Blueprints/Input/Actions/IA_Aim.IA_Aim"))
  ;[1 1 1] Start/Stop Aiming
  (:Triggered
    ;;[1 1 1] Replicates the spine rotation
    (CallFunction|ReplicateAimRot))
  (:Started
    (bind _output_get (Variables|Default|SetbAiming true))
    (CallFunction|SRAiming _output_get)
    (Default|CallOnStartAiming))
  (:Completed
    (bind _output_get_2 (Variables|Default|SetbAiming false))
    (CallFunction|SRAiming _output_get_2)
    (Default|CallOnStopAiming)))

(event Input|EnhancedActionEvents|EnhancedInputActionIA_Shoot
  (params (ActionValue :type Boolean) (ElapsedSeconds :type Float%20%28double-precision%29) (TriggeredSeconds :type Float%20%28double-precision%29) (InputAction :type Input%20Action%20Object%20Reference :default "/Game/VeilstormTasks/Blueprints/Input/Actions/IA_Shoot.IA_Shoot"))
  ;[1 1 1] Shooting ...unrealistic cause the first time a gun is shot is instant
  (if (CallFunction|CanShoot)
    (switch Utilities|FlowControl|Switch|SwitchonE_WeaponFireType (Variables|/Game/VeilstormTasks/Data/DABP_WeaponInfo.DABP_WeaponInfo_C|GetWeaponFireType (Variables|WeaponData|GetWeaponDataAsset))
      (:NewEnumerator6
        (Utilities|AutomaticShooting))
      (:NewEnumerator9
        (Utilities|SingleShooting)))))

(event Input|EnhancedActionEvents|EnhancedInputActionIA_Reload
  (params (ActionValue :type Boolean) (ElapsedSeconds :type Float%20%28double-precision%29) (TriggeredSeconds :type Float%20%28double-precision%29) (InputAction :type Input%20Action%20Object%20Reference :default "/Game/VeilstormTasks/Blueprints/Input/Actions/IA_Reload.IA_Reload"))
  (:Started
    (if (CallFunction|CanReload)
      (Animation|Montage|PlayMontage (Variables|/Script/Engine.Character|GetMesh (Variables|CharacterReferances|GetCharacter)) (Variables|/Game/VeilstormTasks/Data/DABP_WeaponInfo.DABP_WeaponInfo_C|GetReloadAnimation (Variables|WeaponData|GetWeaponDataAsset))
        (:then
          (CallFunction|ServerReload (Variables|/Script/Engine.Character|GetMesh (Variables|CharacterReferances|GetCharacter)) (Variables|/Game/VeilstormTasks/Data/DABP_WeaponInfo.DABP_WeaponInfo_C|GetReloadAnimation (Variables|WeaponData|GetWeaponDataAsset))))))))

(event EventBeginPlay
  (bind _ascharacter (Utilities|Casting|CastToCharacter (Components|GetOwner)))
  (bind _output_get (Variables|CharacterReferances|SetCharacter _ascharacter))
  (if (Utilities|DoesObjectImplementInterface (Components|SkeletalMesh|GetAnimInstance (Variables|/Script/Engine.Character|GetMesh _output_get)) "/Game/VeilstormTasks/Data/BPI_WeaponInterface.BPI_WeaponInterface_C")
    (Variables|CharacterReferances|SetAnimInstance (Components|SkeletalMesh|GetAnimInstance (Variables|/Script/Engine.Character|GetMesh _output_get)))
    (CallFunction|EquipWeapon (Variables|Config|GetInitalWeapon))
    (else
      (Development|PrintString "[Warning] Weapon Compnent: Animation Blueprint Dosn't implement the weapons interface "))))

(event EventEndPlay
  (params (EndPlayReason :type EEndPlayReason%20Enum :default "Destroyed"))
  ;[1 1 1] Cleaning Up At destruction
  (Actor|DestroyActor (Variables|WeaponData|GetCurrentWeapon)))

(event Input|KeyboardEvents|DebugKeyT
  (params (Key :type Key%20Structure :default "None") (ActionValue :type Input%20Action%20Value%20Structure))
  (:Pressed
    (CallFunction|EquipWeapon "/Game/VeilstormTasks/Data/WeaponsDATA/Pistol_DATA.Pistol_DATA")))

(fn EquipWeapon
  (params (WeaponDataAsset :type DABP%20Weapon%20Info%20Object%20Reference))
  (if (not (Variables|Default|GetbEquiped))
    _
    (else
      (Utilities|UnequipWeapon
        (:Done
          _))))
  (bind _output_get (Variables|WeaponData|SetWeaponDataAsset WeaponDataAsset))
  (bind _returnvalue (Game|SpawnActorfromClass (Variables|/Game/VeilstormTasks/Data/DABP_WeaponInfo.DABP_WeaponInfo_C|GetWeaponClass _output_get) (Math|Transform|MakeTransform "0, 0, 0" "0, 0, 0" "1.000000,1.000000,1.000000") "AlwaysSpawn" "MultiplyWithRoot" (Components|GetOwner) 0))
  (bind _asbp_master_weapon (Utilities|Casting|CastToBP_MasterWeapon _returnvalue)
    (:then
      (bind _output_get_2 (Variables|WeaponData|SetCurrentWeapon _asbp_master_weapon))
      (Transformation|AttachComponentToComponent _output_get_2 (Variables|/Script/Engine.Character|GetMesh (Variables|CharacterReferances|GetCharacter)) (Variables|/Game/VeilstormTasks/Data/DABP_WeaponInfo.DABP_WeaponInfo_C|GetSocket (Variables|WeaponData|GetWeaponDataAsset)) "KeepRelative" "KeepRelative" "KeepRelative" true)
      (Class|BPIWeaponInterface|WeaponEquiped(Message) (Components|SkeletalMesh|GetAnimInstance (Variables|/Script/Engine.Character|GetMesh (Variables|CharacterReferances|GetCharacter))) (Variables|WeaponData|GetWeaponDataAsset))
      (Variables|Default|SetbEquiped true)
      (Variables|Default|SetAmmo (Variables|/Game/VeilstormTasks/Data/DABP_WeaponInfo.DABP_WeaponInfo_C|GetIntialAmmo (Variables|WeaponData|GetWeaponDataAsset)))
      (Variables|Default|SetCurrentMag (Variables|/Game/VeilstormTasks/Data/DABP_WeaponInfo.DABP_WeaponInfo_C|GetMagCapacity (Variables|WeaponData|GetWeaponDataAsset))))
    (:CastFailed
      (Development|PrintString "Weapon Class Assigned in WeaponDATA does not inhert from Master Weapon"))))

(fn Shoot
  (bind _returnvalue (Game|GetPlayerCameraManager 0))
  (bind _weapondataasset (Variables|WeaponData|GetWeaponDataAsset))
  (bind _returnvalue_2 (Camera|GetCameraLocation _returnvalue))
  (bind _weaponfireanimation (Variables|/Game/VeilstormTasks/Data/DABP_WeaponInfo.DABP_WeaponInfo_C|GetWeaponFireAnimation _weapondataasset))
  ;[1 1 1] Play the Fire Animation
  (Components|Animation|PlayAnimation (Variables|/Game/VeilstormTasks/Blueprints/Weapons/BP_MasterWeapon.BP_MasterWeapon_C|GetSkeletalMesh (Variables|WeaponData|GetCurrentWeapon)) _weaponfireanimation false)
  (CallFunction|ServerPlayAnim _weaponfireanimation false)
  ;[1 1 1] LineTrace to the center of the screen
  (bind (_outhit _returnvalue_3) (Collision|LineTraceByChannel _returnvalue_2 (+ _returnvalue_2 (* (Transformation|GetActorForwardVector _returnvalue) (Variables|/Game/VeilstormTasks/Data/DABP_WeaponInfo.DABP_WeaponInfo_C|GetShootRange (Variables|WeaponData|GetWeaponDataAsset)))) "TraceTypeQuery1" true 0 "None"))
  (if _returnvalue_3
    (CallFunction|ServerShootLineTrace (Transformation|GetWorldLocation (Variables|/Game/VeilstormTasks/Blueprints/Weapons/BP_MasterWeapon.BP_MasterWeapon_C|GetMuzzlePoint (Variables|WeaponData|GetCurrentWeapon))) (.Location (Collision|BreakHitResult _outhit)) (Variables|CharacterReferances|GetCharacter) (Variables|WeaponData|GetWeaponDataAsset))
    (else
      (CallFunction|ServerReduceMag (Variables|WeaponData|GetWeaponDataAsset)))))

(fn OnRepBAiming
  (bind _character (Variables|CharacterReferances|GetCharacter))
  ;[1 1 1] Can use the turn in place Function from the character instead if there's a decent animation for it
  (Utilities|IsValid _character
    (:Is%20Valid
      (Variables|/Script/Engine.Pawn|SetbUseControllerRotationYaw _character (Variables|Default|GetbAiming))
      (Class|BPIWeaponInterface|IsAiming(Message) (Variables|CharacterReferances|GetAnimInstance) (Variables|Default|GetbAiming)))))

(fn ReplicateAimRot
  (bind _character (Variables|CharacterReferances|GetCharacter))
  (bind _returnvalue (Pawn|GetControlRotation _character :!class /Script/Engine.Pawn))
  (bind _returnvalue_2 (Transformation|GetActorRotation _character))
  (bind _returnvalue_3 (Math|Rotator|Delta(Rotator) _returnvalue _returnvalue_2))
  (CallFunction|ServerRepAimRot (Math|Rotator|MakeRotator (* (.pitch _returnvalue_3) -1.0) 0.0 (Math|Float|Clamp(Float) (.yaw _returnvalue_3) -9e+01 9e+01))))

(fn OnRepAimRotation
  (Class|BPIWeaponInterface|ReplicateAimRot(Message) (Variables|CharacterReferances|GetAnimInstance) (Variables|Default|GetAimRotation)))

(fn ServerDamageCalc
  (params (Start :type Vector) (End :type Vector) (DamageCauser :type Actor%20Object%20Reference))
  (bind _outhit (Collision|LineTraceByChannel Start End "TraceTypeQuery1" true 0 "ForDuration"))
  ;[1 1 1] if the bone hit is not registered in the map deal 10 damage
  (if (.ReturnValue (Utilities|Map|Find (Variables|Default|GetBoneDamageMap) (.HitBoneName (Collision|BreakHitResult _outhit))))
    (Game|Damage|ApplyDamage (.HitActor (Collision|BreakHitResult _outhit)) (.Value (Utilities|Map|Find (Variables|Default|GetBoneDamageMap) (.HitBoneName (Collision|BreakHitResult _outhit)))) 0 DamageCauser)
    (else
      (Game|Damage|ApplyDamage (.HitActor (Collision|BreakHitResult _outhit)) 1e+01 0 DamageCauser))))

(fn ReloadCalc
  (if (<= (Variables|Default|GetAmmo) (Variables|/Game/VeilstormTasks/Data/DABP_WeaponInfo.DABP_WeaponInfo_C|GetMaxAllowedAmmo (Variables|WeaponData|GetWeaponDataAsset)))
    (bind _output_get (LocalVariables|SetMissingMag (- (Variables|/Game/VeilstormTasks/Data/DABP_WeaponInfo.DABP_WeaponInfo_C|GetMagCapacity (Variables|WeaponData|GetWeaponDataAsset)) (Variables|Default|GetCurrentMag))))
    (if (<= _output_get (Variables|Default|GetAmmo))
      (Variables|Default|SetAmmo (- (Variables|Default|GetAmmo) (LocalVariables|GetMissingMag)))
      (Variables|Default|SetCurrentMag (+ (LocalVariables|GetMissingMag) (Variables|Default|GetCurrentMag)))
      (else
        (Variables|Default|SetCurrentMag (+ (Variables|Default|GetCurrentMag) (Variables|Default|GetAmmo)))
        (Variables|Default|SetAmmo 0)))
    (else
      (Development|PrintString "Cheater Detected!  ammo > MaxAmmo"))))

(fn ReduceMag
  (if (<= (Variables|Default|GetCurrentMag) (Variables|/Game/VeilstormTasks/Data/DABP_WeaponInfo.DABP_WeaponInfo_C|GetMagCapacity (Variables|WeaponData|GetWeaponDataAsset)))
    (if (> (Variables|Default|GetCurrentMag) 0)
      (Math|Integer|DecrementInt (Variables|Default|GetCurrentMag)))
    (else
      (Development|PrintString "Cheater! Mag > Mag capacity"))))

(fn CanShoot
  (return (Math|Boolean|ANDBoolean (> (Variables|Default|GetCurrentMag) 0) (not (Variables|Default|GetbReloading)) (Variables|Default|GetbAiming))))

(fn CanReload
  (return (and (< (Variables|Default|GetCurrentMag) (Variables|/Game/VeilstormTasks/Data/DABP_WeaponInfo.DABP_WeaponInfo_C|GetMagCapacity (Variables|WeaponData|GetWeaponDataAsset))) (> (Variables|Default|GetAmmo) 0))))