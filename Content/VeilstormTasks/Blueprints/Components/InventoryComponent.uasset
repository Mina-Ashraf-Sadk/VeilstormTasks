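; Character inventory component that manages primary, secondary and unarmed weapon slots and forwards aim, shoot, reload and special-action input to the equipped weapon.
; On BeginPlay, if the AnimBP implements the weapon interface, server RPCs spawn the starting weapons onto holster sockets.
; Slot switches apply locally and via server multicast, swapping socket attachments and sending weapon data to the AnimBP.
; EndPlay destroys all three weapons through a server RPC.
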(event Custom|Server_Cleanup
  ;[1 0 0] Destructor (EndPlay)
  (Actor|DestroyActor (Variables|Unarmed|GetUnarmedWeapon))
  (Actor|DestroyActor (Variables|PrimaryWeapon|GetPrimaryWeapon))
  (Actor|DestroyActor (Variables|SecondaryWeapon|GetSecondaryWeapon)))

(event Custom|MultiCast_SetActiveSlot
  (params (ActiveWeaponSlot :type E_WeaponSlotType%20Enum :default "NewEnumerator6"))
  ;[1 0.03179 0] RPCs
  ;;[1 1 1] Change Active Weapon
  (CallFunction|SetActiveWeaponSlot ActiveWeaponSlot))

(event Custom|Server_SetUnarmedWeapon
  (params (WeaponClass :type BP%20Unarmed%20Class%20Reference))
  ;[1 0.03179 0] RPCs
  ;;[1 1 1] Give Weapons
  (CallFunction|SetUnarmed WeaponClass))

(event Custom|Server_SetActiveSlot
  (params (WeaponSlot :type E_WeaponSlotType%20Enum :default "NewEnumerator6"))
  ;[1 0.03179 0] RPCs
  ;;[1 1 1] Change Active Weapon
  (CallFunction|MultiCastSetActiveSlot WeaponSlot))

(event Custom|Server_ChangePrimaryWeapon
  (params (WeaponClass :type BP%20Primary%20Weapon%20Class%20Reference))
  ;[1 0.03179 0] RPCs
  ;;[1 1 1] Give Weapons
  (CallFunction|SetPrimaryWeapon WeaponClass))

(event Custom|Server_ChangeSecondaryWeapon
  (params (WeaponClass :type BP%20Secondary%20Weapon%20Class%20Reference))
  ;[1 0.03179 0] RPCs
  ;;[1 1 1] Give Weapons
  (CallFunction|SetSecondaryWeapon WeaponClass))

(event Input|EnhancedActionEvents|EnhancedInputActionIA_EquipPrimary
  (params (ActionValue :type Boolean) (ElapsedSeconds :type Float%20%28double-precision%29) (TriggeredSeconds :type Float%20%28double-precision%29) (InputAction :type Input%20Action%20Object%20Reference :default "/Game/VeilstormTasks/Blueprints/Input/Actions/IA_EquipPrimary.IA_EquipPrimary"))
  ;[0 0.1216 1] input Actions
  ;;[1 1 1] Cycle through Weapons
  (:Started
    (CallFunction|SetActiveWeaponSlot "NewEnumerator6")
    (CallFunction|ServerSetActiveSlot "NewEnumerator6")))

(event Input|EnhancedActionEvents|EnhancedInputActionIA_EquipSecondary
  (params (ActionValue :type Boolean) (ElapsedSeconds :type Float%20%28double-precision%29) (TriggeredSeconds :type Float%20%28double-precision%29) (InputAction :type Input%20Action%20Object%20Reference :default "/Game/VeilstormTasks/Blueprints/Input/Actions/IA_EquipSecondary.IA_EquipSecondary"))
  ;[0 0.1216 1] input Actions
  ;;[1 1 1] Cycle through Weapons
  (:Started
    (CallFunction|SetActiveWeaponSlot "NewEnumerator7")
    (CallFunction|ServerSetActiveSlot "NewEnumerator7")))

(event Input|EnhancedActionEvents|EnhancedInputActionIA_EquipUnarmed
  (params (ActionValue :type Boolean) (ElapsedSeconds :type Float%20%28double-precision%29) (TriggeredSeconds :type Float%20%28double-precision%29) (InputAction :type Input%20Action%20Object%20Reference :default "/Game/VeilstormTasks/Blueprints/Input/Actions/IA_EquipUnarmed.IA_EquipUnarmed"))
  ;[0 0.1216 1] input Actions
  ;;[1 1 1] Cycle through Weapons
  (:Started
    (CallFunction|SetActiveWeaponSlot "NewEnumerator9")
    (CallFunction|ServerSetActiveSlot "NewEnumerator9")))

(event Input|EnhancedActionEvents|EnhancedInputActionIA_Shoot
  (params (ActionValue :type Boolean) (ElapsedSeconds :type Float%20%28double-precision%29) (TriggeredSeconds :type Float%20%28double-precision%29) (InputAction :type Input%20Action%20Object%20Reference :default "/Game/VeilstormTasks/Blueprints/Input/Actions/IA_Shoot.IA_Shoot"))
  (bind _equipedweapon (Variables|Configuration|GetEquipedWeapon))
  ;[0 0.1216 1] input Actions
  (:Started
    (Default|StartShooting _equipedweapon))
  (:Completed
    (Default|StopShooting _equipedweapon)))

(event Input|EnhancedActionEvents|EnhancedInputActionIA_Reload
  (params (ActionValue :type Boolean) (ElapsedSeconds :type Float%20%28double-precision%29) (TriggeredSeconds :type Float%20%28double-precision%29) (InputAction :type Input%20Action%20Object%20Reference :default "/Game/VeilstormTasks/Blueprints/Input/Actions/IA_Reload.IA_Reload"))
  (bind _equipedweapon (Variables|Configuration|GetEquipedWeapon))
  ;[0 0.1216 1] input Actions
  (:Started
    (Default|StartReload _equipedweapon))
  (:Completed
    (Default|StopReload _equipedweapon)))

(event Input|EnhancedActionEvents|EnhancedInputActionIA_Aim
  (params (ActionValue :type Boolean) (ElapsedSeconds :type Float%20%28double-precision%29) (TriggeredSeconds :type Float%20%28double-precision%29) (InputAction :type Input%20Action%20Object%20Reference :default "/Game/VeilstormTasks/Blueprints/Input/Actions/IA_Aim.IA_Aim"))
  (bind _equipedweapon (Variables|Configuration|GetEquipedWeapon))
  ;[0 0.1216 1] input Actions
  (:Started
    (Default|StartAim _equipedweapon))
  (:Completed
    (Default|StopAim _equipedweapon)))

(event Input|EnhancedActionEvents|EnhancedInputActionIA_WeaponSpeicalAction
  (params (ActionValue :type Boolean) (ElapsedSeconds :type Float%20%28double-precision%29) (TriggeredSeconds :type Float%20%28double-precision%29) (InputAction :type Input%20Action%20Object%20Reference :default "/Game/VeilstormTasks/Blueprints/Input/Actions/IA_WeaponSpeicalAction.IA_WeaponSpeicalAction"))
  (bind _equipedweapon (Variables|Configuration|GetEquipedWeapon))
  ;[0 0.1216 1] input Actions
  (:Started
    (Default|StartSpeicalAction _equipedweapon))
  (:Completed
    (Default|StopSpeicalAction _equipedweapon)))

(event EventEndPlay
  (params (EndPlayReason :type EEndPlayReason%20Enum :default "Destroyed"))
  ;[1 0 0] Destructor (EndPlay)
  (CallFunction|ServerCleanup))

(event EventBeginPlay
  ;[1 1 1] Constructor (BeginPlay)
  (bind _ascharacter (Utilities|Casting|CastToCharacter (Components|GetOwner)))
  (bind _output_get (Variables|Configuration|SetCharacter _ascharacter))
  (if (Utilities|DoesObjectImplementInterface (Components|SkeletalMesh|GetAnimInstance (Variables|/Script/Engine.Character|GetMesh _output_get)) "/Game/VeilstormTasks/Data/BPI_WeaponAnimationInterface.BPI_WeaponAnimationInterface_C")
    (CallFunction|WeaponsInitialization)
    (else
      (Development|PrintString "[Warning] Weapon Compnent: Animation Blueprint Dosn't implement the weapons interface "))))

(fn SetSecondaryWeapon
  (params (WeaponClass :type BP%20Secondary%20Weapon%20Class%20Reference))
  (Utilities|IsValid (Variables|SecondaryWeapon|GetSecondaryWeapon)
    (:Is%20Valid
      (Actor|DestroyActor (Variables|SecondaryWeapon|GetSecondaryWeapon)))
    (:Is%20Not%20Valid
      _))
  (bind _returnvalue (Game|SpawnActorfromClass WeaponClass (Math|Transform|MakeTransform "0, 0, 0" "0, 0, 0" "1.000000,1.000000,1.000000") "AlwaysSpawn" "MultiplyWithRoot" (Variables|Configuration|GetCharacter) 0))
  (Variables|SecondaryWeapon|SetSecondaryWeapon _returnvalue)
  (Transformation|AttachComponentToComponent (Variables|SecondaryWeapon|GetSecondaryWeapon) (Variables|/Script/Engine.Character|GetMesh (Variables|Configuration|GetCharacter)) (Variables|/Game/VeilstormTasks/Data/DABP_WeaponInfo.DABP_WeaponInfo_C|GetHostlerSocket (Variables|/Game/VeilstormTasks/Blueprints/Weapons/MasterClasses/BP_MasterWeapon.BP_MasterWeapon_C|GetWeaponDATA (Variables|SecondaryWeapon|GetSecondaryWeapon))) "KeepRelative" "KeepRelative" "KeepRelative" true))

(fn SetPrimaryWeapon
  (params (WeaponClass :type BP%20Primary%20Weapon%20Class%20Reference))
  (Utilities|IsValid (Variables|PrimaryWeapon|GetPrimaryWeapon)
    (:Is%20Valid
      (Actor|DestroyActor (Variables|PrimaryWeapon|GetPrimaryWeapon)))
    (:Is%20Not%20Valid
      _))
  (bind _returnvalue (Game|SpawnActorfromClass WeaponClass (Math|Transform|MakeTransform "0, 0, 0" "0, 0, 0" "1.000000,1.000000,1.000000") "AlwaysSpawn" "MultiplyWithRoot" (Variables|Configuration|GetCharacter) 0))
  (Variables|PrimaryWeapon|SetPrimaryWeapon _returnvalue)
  (Transformation|AttachComponentToComponent (Variables|PrimaryWeapon|GetPrimaryWeapon) (Variables|/Script/Engine.Character|GetMesh (Variables|Configuration|GetCharacter)) (Variables|/Game/VeilstormTasks/Data/DABP_WeaponInfo.DABP_WeaponInfo_C|GetHostlerSocket (Variables|/Game/VeilstormTasks/Blueprints/Weapons/MasterClasses/BP_MasterWeapon.BP_MasterWeapon_C|GetWeaponDATA (Variables|PrimaryWeapon|GetPrimaryWeapon))) "KeepRelative" "KeepRelative" "KeepRelative" true))

(fn SetUnarmed
  (params (WeaponClass :type BP%20Unarmed%20Class%20Reference))
  (Utilities|IsValid (Variables|Unarmed|GetUnarmedWeapon)
    (:Is%20Valid
      (Actor|DestroyActor (Variables|Unarmed|GetUnarmedWeapon)))
    (:Is%20Not%20Valid
      _))
  (bind _returnvalue (Game|SpawnActorfromClass (Variables|Unarmed|GetFirstUnarmedWeapon) (Math|Transform|MakeTransform "0, 0, 0" "0, 0, 0" "1.000000,1.000000,1.000000") "AlwaysSpawn" "MultiplyWithRoot" (Variables|Configuration|GetCharacter) 0))
  (Variables|Unarmed|SetUnarmedWeapon _returnvalue)
  (Transformation|AttachComponentToComponent (Variables|Unarmed|GetUnarmedWeapon) (Variables|/Script/Engine.Character|GetMesh (Variables|Configuration|GetCharacter)) (Variables|/Game/VeilstormTasks/Data/DABP_WeaponInfo.DABP_WeaponInfo_C|GetHostlerSocket (Variables|/Game/VeilstormTasks/Blueprints/Weapons/MasterClasses/BP_MasterWeapon.BP_MasterWeapon_C|GetWeaponDATA (Variables|Unarmed|GetUnarmedWeapon))) "KeepRelative" "KeepRelative" "KeepRelative" true))

(fn WeaponsInitialization
  ;[1 1 1] Initialization
  (CallFunction|ServerChangeSecondaryWeapon (Variables|SecondaryWeapon|GetFirstSecondaryWeapon))
  (CallFunction|ServerChangePrimaryWeapon (Variables|PrimaryWeapon|GetFirstPrimaryWeapon))
  (CallFunction|ServerSetUnarmedWeapon (Variables|Unarmed|GetFirstUnarmedWeapon))
  (CallFunction|ServerSetActiveSlot "NewEnumerator9")
  (CallFunction|SetActiveWeaponSlot (Variables|Configuration|GetActiveWeaponSlot)))

(fn SetActiveWeaponSlot
  (params (ActiveWeaponSlot :type E_WeaponSlotType%20Enum :default "NewEnumerator6"))
  (Variables|Configuration|SetActiveWeaponSlot ActiveWeaponSlot)
  (Utilities|IsValid (Variables|Configuration|GetEquipedWeapon)
    (:Is%20Valid
      ;[1 1 1] Hostle the current weapon if exists
      (Transformation|AttachComponentToComponent (Variables|Configuration|GetEquipedWeapon) (Variables|/Script/Engine.Character|GetMesh (Variables|Configuration|GetCharacter)) (Variables|/Game/VeilstormTasks/Data/DABP_WeaponInfo.DABP_WeaponInfo_C|GetHostlerSocket (Variables|/Game/VeilstormTasks/Blueprints/Weapons/MasterClasses/BP_MasterWeapon.BP_MasterWeapon_C|GetWeaponDATA (Variables|Configuration|GetEquipedWeapon))) "KeepRelative" "KeepRelative" "KeepRelative" true))
    (:Is%20Not%20Valid
      _))
  ;[1 1 1] Set the new active weapon slot
  (bind _output_get (Variables|Configuration|SetEquipedWeapon (Utilities|Select :Index (Variables|Configuration|GetActiveWeaponSlot) :NewEnumerator6 (Variables|PrimaryWeapon|GetPrimaryWeapon) :NewEnumerator7 (Variables|SecondaryWeapon|GetSecondaryWeapon) :NewEnumerator9 (Variables|Unarmed|GetUnarmedWeapon))))
  (Utilities|IsValid _output_get
    (:Is%20Valid
      ;[1 1 1] Equip the new weapon
      (Transformation|AttachComponentToComponent (Variables|Configuration|GetEquipedWeapon) (Variables|/Script/Engine.Character|GetMesh (Variables|Configuration|GetCharacter)) (Variables|/Game/VeilstormTasks/Data/DABP_WeaponInfo.DABP_WeaponInfo_C|GetSocket (Variables|/Game/VeilstormTasks/Blueprints/Weapons/MasterClasses/BP_MasterWeapon.BP_MasterWeapon_C|GetWeaponDATA (Variables|Configuration|GetEquipedWeapon))) "KeepRelative" "KeepRelative" "KeepRelative" true)
      (Class|BPIWeaponAnimationInterface|WeaponEquiped(Message) (Components|SkeletalMesh|GetAnimInstance (Variables|/Script/Engine.Character|GetMesh (Variables|Configuration|GetCharacter))) (Variables|/Game/VeilstormTasks/Blueprints/Weapons/MasterClasses/BP_MasterWeapon.BP_MasterWeapon_C|GetWeaponDATA (Variables|Configuration|GetEquipedWeapon)))
      (Development|PrintString (Utilities|GetDisplayName (Variables|Configuration|GetCharacter))))))