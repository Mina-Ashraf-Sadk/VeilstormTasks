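; Replicated actor component for a multiplayer teleport ability with cooldown, effects and camera shake.
; StartTeleport runs a looping timer that steps a debug-sphere target along control rotation, ground-tracing for walkable floor until EndTeleport or an invalid step fires the teleport.
; The owning client predicts the move while the server validates range and cooldown, then multicasts it or corrects the client.
; A debug key fakes a destination to test reconciliation; line-of-sight validation is disconnected.
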(event Custom|Multicast_EndTeleport
  (params (NewLocation :type Vector) (Instigator :type Controller%20Object%20Reference))
  ;[0 0 0] Multicast
  ;;[1 1 1] Update all clients on players teleport
  (Teleport|Mechanics|PerformTeleport NewLocation)
  (Utilities|IsRemotePlayer Instigator
    (:Remote
      (Teleport|Effects|SpawnTeleportEffects false false NewLocation))))

(event Custom|Server_RequestTeleport
  (params (ProposedLocation :type Vector) (Instigator :type Controller%20Object%20Reference))
  ;[0 0 0] Server
  ;;[1 1 1] Server - Request teleport, validate proposed location from client
  (bind _bisvalid (Teleport|Utility|ValidateTeleportDestination ProposedLocation))
  (if _bisvalid
    (CallFunction|MulticastStartTeleport Instigator)
    (Utilities|FlowControl|Delay (Variables|Teleport|Configuration|GetTeleportDuration))
    (CallFunction|MulticastEndTeleport ProposedLocation Instigator)
    (else
      (CallFunction|ClientCorrectPosition (Transformation|GetActorLocation (Components|GetOwner))))))

(event Custom|Client_CorrectPosition
  (params (CorrectPosition :type Vector))
  ;[0 0 0] Client
  ;;[1 1 1] Client - Reconcile correct position based on server validation
  (bind _output_get (Variables|Teleport|Status|SetLastValidTeleportLocation CorrectPosition))
  (Teleport|Mechanics|PerformTeleport _output_get))

(event Custom|Client_TryCheat
  ;[0 0 0] Input
  ;;[1 1 1] Cheat command (test server reconcilation)
  (Variables|Teleport|Status|SetLastValidTeleportLocation "2180.000000,700.000000,200.000000")
  (Teleport|Mechanics|EndTeleport))

(event Custom|Client_PerformTeleport
  (params (Location :type Vector))
  ;[0 0 0] Client
  ;;[1 1 1] Client - Perform teleport prediction
  (Variables|Teleport|Status|SetLastValidTeleportLocation Location)
  (Teleport|Effects|SpawnTeleportEffects true true (Transformation|GetActorLocation (Components|GetOwner)))
  (Variables|Teleport|Status|SetbIsOnCooldown true)
  (Teleport|Effects|PlayCameraShake)
  (Utilities|FlowControl|Delay (Variables|Teleport|Configuration|GetTeleportDuration))
  (Teleport|Mechanics|PerformTeleport (Variables|Teleport|Status|GetLastValidTeleportLocation))
  (Teleport|Effects|SpawnTeleportEffects false false (Variables|Teleport|Status|GetLastValidTeleportLocation)))

(event Custom|Multicast_StartTeleport
  (params (Instigator :type Controller%20Object%20Reference))
  ;[0 0 0] Multicast
  ;;[1 1 1] Toggle player visibility
  (Utilities|IsRemotePlayer Instigator
    (:Remote
      (Teleport|Effects|SpawnTeleportEffects true true (Transformation|GetActorLocation (Components|GetOwner))))))

(event Custom|StartCooldown
  ;[0 0 0] Server
  ;;[1 1 1] Cooldown
  (Variables|Teleport|Status|SetbIsOnCooldown true)
  (if (Variables|Teleport|Status|GetbIsOnCooldown)
    (Utilities|Time|SetTimerbyFunctionName 0 "ResetCooldown" (Variables|Teleport|Configuration|GetCooldownDuration))))

(event EventBeginPlay
  ;[0 0 0] Begin play
  ;;[1 1 1] Set component to replicate
  (Class|ActorComponent|SetIsReplicated true))

(event Input|KeyboardEvents|DebugKeyC
  (params (Key :type Key%20Structure) (ActionValue :type Input%20Action%20Value%20Structure))
  ;[0 0 0] Input
  ;;[1 1 1] Cheat command (test server reconcilation)
  (:Pressed
    (CallFunction|ClientTryCheat)))

(fn CanTeleportto
  (params (Destination :type Hit%20Result%20Structure))
  (bind (_bblockinghit _binitialoverlap _time _distance _location _impactpoint _normal _impactnormal) (Collision|BreakHitResult Destination))
  (return (and _bblockinghit (> (.Z (Math|Vector|BreakVector _impactnormal)) 0.7)) _location))

(fn CalculateTeleportDestination
  (params (StartLocation :type Vector) (ForwardVector :type Vector))
  ;[1 1 1] Calculates next end location based on previous valid teleport location. Uses Capsule radius as spacing
  (LocalVariables|SetEndLocation (+ (Variables|Teleport|Status|GetLastValidTeleportLocation) (* ForwardVector (* (Variables|Teleport|Configuration|GetCapsuleRadius) 2.0))))
  (if (< (Math|Vector|VectorLength (- (LocalVariables|GetEndLocation) StartLocation)) (Variables|Teleport|Configuration|GetMaxTeleportDistance))
    ;[1 1 1] Traces at end location to find floor.
    (bind _outhit (Teleport|Calculations|PerformGroundTrace (LocalVariables|GetEndLocation)))
    ;[1 1 1] Runs checks to see if it's a walkable surface
    (bind (_bcanteleport _location) (Teleport|Utility|CanTeleportto _outhit))
    (if _bcanteleport
      (return _location)
      (else
        _)))
  (return "0, 0, 0"))

(fn StartTeleport
  ;[1 1 1] Zeros out teleport location
  (Variables|Teleport|Status|SetLastValidTeleportLocation "0, 0, 0")
  ;[1 1 1] Checks cooldown is innactive
  (Utilities|IsCooldownActive
    (:Innactive
      ;[1 1 1] Store the location when initially casting the teleport ability
      (Variables|Teleport|Status|SetLastValidTeleportLocation (Transformation|GetActorLocation (Components|GetOwner)))
      ;[1 1 1] Updates the teleport location based on the orb speed, whilst the user is holding down the key
      (Utilities|Time|SetTimerbyFunctionName 0 "UpdateTeleportDestination" (Variables|Teleport|Configuration|GetTeleportOrbSpeed) true)
      ;[1 1 1] Premature function call to skip the Teleport Orb Speed delay
      (Teleport|Mechanics|UpdateTeleportDestination))))

(fn EndTeleport
  ;[1 1 1] Checks that we have a valid target location
  (if (not (Math|Vector|VectorIsZero (Variables|Teleport|Status|GetLastValidTeleportLocation)))
    ;[1 1 1] Checks cooldown is innactive
    (Utilities|IsCooldownActive
      (:Innactive
        ;[1 1 1] Clears teleport location orb timer
        (Utilities|Time|ClearTimerbyFunctionName 0 "UpdateTeleportDestination")
        (Utilities|FlowControl|Sequence
          (:then_0
            (Networking|SwitchHasAuthority
              (:Authority
                ;[1 1 1] Server
                (CallFunction|ServerRequestTeleport (Variables|Teleport|Status|GetLastValidTeleportLocation) (Teleport|Accessors|GetInstigatorController))
                ;;[1 1 1] Not a great solution by any means, if the teleport location isn't valid, it still triggers.
                (Teleport|Effects|PlayCameraShake))
              (:Remote
                ;[1 1 1] Client
                ;;[1 1 1] Client prediction to stay responsive
                (CallFunction|ClientPerformTeleport (Variables|Teleport|Status|GetLastValidTeleportLocation))
                ;;[1 1 1] Immediately called on the server for validation and reconcilation.
                (CallFunction|ServerRequestTeleport (Variables|Teleport|Status|GetLastValidTeleportLocation) (Teleport|Accessors|GetInstigatorController)))))
          (:then_1
            ;[1 1 1] Initiates cooldown timer
            (CallFunction|StartCooldown)))))))

(fn UpdateTeleportDestination
  (bind _returnvalue (Components|GetOwner))
  (bind _instigator (Variables|/Script/Engine.Actor|GetInstigator _returnvalue))
  (bind _returnvalue_2 (Pawn|GetControlRotation _instigator :!class /Script/Engine.Pawn))
  (bind _returnvalue_3 (Math|Vector|GetForwardVector _returnvalue_2))
  ;[1 1 1] Calculates a valid teleport location
  (bind _calculatedlocation (Teleport|Calculations|CalculateTeleportDestination (Transformation|GetActorLocation _returnvalue) (Math|Vector|MakeVectorNetQuantize (.x _returnvalue_3) (.y _returnvalue_3) 0.0)))
  ;[1 1 1] Checking location is valid and not null
  (if (not (Math|Vector|VectorIsZero _calculatedlocation))
    (bind _output_get (Variables|Teleport|Status|SetLastValidTeleportLocation _calculatedlocation))
    (Rendering|Debug|DrawDebugSphere _output_get 2e+01 12 "(R=0.000000,G=0.000000,B=1.000000,A=1.000000)" 0.2 1.0)
    (else
      ;[1 1 1] If location is invalid, orb timer is stopped and we're teleported to the final destination
      (Teleport|Mechanics|EndTeleport))))

(fn PerformTeleport
  (params (NewLocation :type Vector))
  ;[1 1 1] Just updates player location based on given vector
  (Transformation|SetActorLocation (Components|GetOwner) NewLocation false true))

(fn PerformGroundTrace
  (params (Start :type Vector))
  ;[1 1 1] Runs trace from given location straight down.
  (bind _outhit (Collision|CapsuleTraceByChannel (+ Start "0.000000,0.000000,1000.000000") (- Start "0.000000,0.000000,1000.000000") (Variables|Teleport|Configuration|GetCapsuleRadius) (Variables|Teleport|Configuration|GetCapsuleHeight) "TraceTypeQuery1" false 0 "None"))
  (return _outhit))

(fn SpawnTeleportEffects
  (params (bPlayAudio :type Boolean) (bPlayerHidden :type Boolean) (Location :type Vector))
  (Utilities|FlowControl|Sequence
    (:then_0
      ;[1 1 1] Visual FX
      (bind _teleporteffect (Variables|Teleport|Effects|GetTeleportEffect)
        (:then
          (Niagara|SpawnSystematLocation _teleporteffect Location))
        (:else)))
    (:then_1
      ;[1 1 1] Audio FX
      (if bPlayAudio
        (bind _teleportsound (Variables|Teleport|Effects|GetTeleportSound)
          (:then
            (Audio|PlaySoundatLocation _teleportsound Location "0, 0, 0" 1.0 1.0 0.0 0 0 0 0))
          (:else))))
    (:then_2
      ;[1 1 1] Player visibility
      (Rendering|SetActorHiddenInGame (Components|GetOwner) bPlayerHidden))))

(fn ValidateTeleportDestination
  (params (ProposedLocation :type Vector))
  (return (Math|Boolean|ANDBoolean (<= (Math|Vector|VectorLength (- ProposedLocation (Transformation|GetActorLocation (Components|GetOwner)))) (Variables|Teleport|Configuration|GetMaxTeleportDistance)) (not false) (not (Variables|Teleport|Status|GetbIsOnCooldown)))))

(fn GetInstigatorController
  ;[1 1 1] Need to compare controllers, given we have access to the components instigator we can get the controller from that.
  (return (Pawn|GetController (Variables|/Script/Engine.Actor|GetInstigator (Components|GetOwner)))))

(fn ResetCooldown
  ;[1 1 1] Sets cooldown to false when cooldown timer runs out.
  (Variables|Teleport|Status|SetbIsOnCooldown false))

(fn PlayCameraShake
  (bind _teleportshake (Variables|Teleport|Effects|GetTeleportShake)
    (:then
      (Class|LegacyCameraShake|StartLegacyCameraShake (Game|GetPlayerCameraManager 0) _teleportshake 5.0 "CameraLocal" "0, 0, 0"))
    (:else)))