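; BP_SpawnPoint is a level-placed spawn location that registers itself with the GM_Map1 game mode and tracks when it becomes free.
; On BeginPlay it adds itself uniquely to the game mode's SpawnLocations array.
; When an actor tagged Player leaves its Box collision, a server-named event adds a "Free" actor tag to mark the point as available.
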(event OnComponentEndOverlap(Box)
  (params (OverlappedComponent :type Primitive%20Component%20Object%20Reference) (OtherActor :type Actor%20Object%20Reference) (OtherComp :type Primitive%20Component%20Object%20Reference) (OtherBodyIndex :type Integer))
  (if (Actor|ActorHasTag OtherActor "Player")
    (CallFunction|ServerMarkasFree)))

(event Custom|Server_MarkAsFree
  (Utilities|Array|Add (Variables|Actor|GetTags) "Free"))

(event EventBeginPlay
  (bind _asgm_map_1 (Utilities|Casting|CastToGM_Map1 (Game|GetGameMode)))
  (Utilities|Array|AddUnique (Variables|/Game/VeilstormTasks/Blueprints/Core/GM_Map1.GM_Map1_C|GetSpawnLocations _asgm_map_1) self))

(fn ConstructionScript)