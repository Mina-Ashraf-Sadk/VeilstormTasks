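; DeathDrop is a level actor that spawns a pair of pickups where it is placed or spawned, presumably as loot left by a death.
; On BeginPlay, only the authority spawns two Pickup actors of different types, one at its own transform and the other offset diagonally.
; The offset pickup is validity-checked and has its mesh swapped to the rocket launcher pickup.
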(event EventBeginPlay
  (bind _returnvalue (Transformation|GetActorTransform))
  (Networking|SwitchHasAuthority
    (:Authority
      (bind _returnvalue_2 (Game|SpawnActorfromClass "/Game/VeilstormTasks/Blueprints/LevelActors/Pickup.Pickup_C" (Transformation|GetActorTransform) "AlwaysSpawn" "MultiplyWithRoot" 0 0))
      (Variables|/Game/VeilstormTasks/Blueprints/LevelActors/Pickup.Pickup_C|SetPickupType _returnvalue_2 "NewEnumerator4")
      (bind _returnvalue_3 (Game|SpawnActorfromClass "/Game/VeilstormTasks/Blueprints/LevelActors/Pickup.Pickup_C" (Math|Transform|MakeTransform (+ (.location _returnvalue) "100.000000,100.000000,0.000000") (.rotation _returnvalue) (.scale _returnvalue)) "AlwaysSpawn" "MultiplyWithRoot" 0 0))
      (Utilities|IsValid _returnvalue_3
        (:Is%20Valid
          (Variables|/Game/VeilstormTasks/Blueprints/LevelActors/Pickup.Pickup_C|SetPickupType _returnvalue_3 "NewEnumerator3")
          (Components|StaticMesh|SetStaticMesh (Variables|/Game/VeilstormTasks/Blueprints/LevelActors/Pickup.Pickup_C|GetStaticMesh _returnvalue_3) "/Game/MilitaryWeapSilver/Pickups/RocketLauncher_Pickup.RocketLauncher_Pickup"))))))

(fn ConstructionScript)