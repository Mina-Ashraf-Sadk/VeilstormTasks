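; Pickup is a placeable level actor that grants health or ammo when an actor overlaps its box.
; A PickupType enum chooses the mesh in the construction script and the message sent on overlap.
; The overlapping actor receives the fixed amount through BPI_PickupInterface, then the pickup destroys itself.
; Actors without that interface only trigger a debug print and leave the pickup in place.
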(event OnComponentBeginOverlap(Box)
  (params (OverlappedComponent :type Primitive%20Component%20Object%20Reference) (OtherActor :type Actor%20Object%20Reference) (OtherComp :type Primitive%20Component%20Object%20Reference) (OtherBodyIndex :type Integer) (bFromSweep :type Boolean) (SweepResult :type Hit%20Result%20Structure%20%28by%20ref%29))
  (bind _output_get (Variables|Default|SetOverlappedActor OtherActor))
  (if (Utilities|DoesObjectImplementInterface _output_get "/Game/VeilstormTasks/Data/BPI_PickupInterface.BPI_PickupInterface_C")
    (switch Utilities|FlowControl|Switch|SwitchonE_PickupType (Variables|Default|GetPickupType)
      (:NewEnumerator3
        (Class|BPIPickupInterface|OnHealthPickup(Message) (Variables|Default|GetOverlappedActor) 25.0))
      (:NewEnumerator4
        (Class|BPIPickupInterface|OnAmmoPickup(Message) (Variables|Default|GetOverlappedActor) 50)))
    (Actor|DestroyActor)
    (else
      (Development|PrintString "Actor Doesn't implement the pickup interface"))))

(fn ConstructionScript
  (switch Utilities|FlowControl|Switch|SwitchonE_PickupType (Variables|Default|GetPickupType)
    (:NewEnumerator3
      (Components|StaticMesh|SetStaticMesh (Variables|Default|GetStaticMesh) "/Game/VeilstormTasks/Art/BasicShapes/SM_ChamferCube.SM_ChamferCube"))
    (:NewEnumerator4
      (Components|StaticMesh|SetStaticMesh (Variables|Default|GetStaticMesh) "/Game/MilitaryWeapSilver/Pickups/AssaultRifle_Pickup.AssaultRifle_Pickup"))))