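; GM_Map1 is the game mode for Map 1, admitting joining players up to a map capacity and spawning them into two teams.
; PostLogin sends players over capacity to a LeaveSession kick, noted as not working.
; Others get a T1 or T2 controller tag for the smaller team, then possess a third-person character spawned at that team's spawn point.
; Spawn points are claimed by removing their "Free" tag, with world origin as fallback.
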(event EventPostLogin
  (params (NewPlayer :type Player%20Controller%20Object%20Reference))
  (CallFunction|HandleNewPlayer NewPlayer))

(fn ConstructionScript)

(fn HandleNewPlayer
  (params (NewPlayer :type Player%20Controller%20Object%20Reference%20%28by%20ref%29))
  (if (< (Utilities|Array|Length (Variables|Game|GetPlayers)) (Variables|Default|GetMapCapacity))
    ;[1 1 1] Spawn Player and add to players list
    (CallFunction|SpawnPlayer NewPlayer)
    (Utilities|Array|AddUnique (Variables|Game|GetPlayers) NewPlayer)
    (else
      ;[1 1 1] should kick player but currently not working
      (CallFunction|KickPlayer NewPlayer))))

(fn KickPlayer
  (params (Player :type Player%20Controller%20Object%20Reference%20%28by%20ref%29))
  (bind _aspc_veilstorm_tasks_controller (Utilities|Casting|CastToPC_VeilstormTasksController Player))
  (Default|LeaveSession _aspc_veilstorm_tasks_controller))

(fn SpawnPlayer
  (params (PlayerToSpawn :type Player%20Controller%20Object%20Reference))
  (CallFunction|AutoAssigntoTeam PlayerToSpawn)
  (bind _availablespawnlocation (CallFunction|FetchSpawnLocation PlayerToSpawn))
  (bind _returnvalue (Game|SpawnActorfromClass "/Game/VeilstormTasks/Core/BP_ThirdPersonCharacter.BP_ThirdPersonCharacter_C" _availablespawnlocation "Undefined" "MultiplyWithRoot" PlayerToSpawn 0))
  (Pawn|Possess PlayerToSpawn _returnvalue))

(fn AutoAssigntoTeam
  (params (PlayerController :type Player%20Controller%20Object%20Reference))
  (bind _tags (Variables|/Script/Engine.Actor|GetTags PlayerController))
  (bind (_team1players _team2players) (|CalculatesTheNumberOfPlayersInEachTeam)
    (:Completed
      (if (<= _team1players _team2players)
        (Utilities|Array|Add _tags "T1")
        (else
          (Utilities|Array|Add _tags "T2"))))))

(fn FetchSpawnLocation
  (params (PlayerController :type Player%20Controller%20Object%20Reference))
  (if (Actor|ActorHasTag PlayerController "T2")
    (bind _outactors (Actor|GetAllActorsOfClasswithTag "/Game/VeilstormTasks/Core/ActorsBP/BP_Team2_SpawnPoint.BP_Team2_SpawnPoint_C" "Free"))
    (bind _output_get (LocalVariables|SetSpawnPoint (Utilities|Array|Get(acopy) _outactors)))
    (Utilities|Array|RemoveItem (Variables|/Script/Engine.Actor|GetTags _output_get) "Free")
    (else
      (bind _outactors_2 (Actor|GetAllActorsOfClasswithTag "/Game/VeilstormTasks/Core/ActorsBP/BP_Team1_SpawnPoint.BP_Team1_SpawnPoint_C" "Free"))
      (bind _output_get_2 (LocalVariables|SetSpawnPoint (Utilities|Array|Get(acopy) _outactors_2)))
      (Utilities|Array|RemoveItem (Variables|/Script/Engine.Actor|GetTags _output_get_2) "Free")))
  (Utilities|IsValid (LocalVariables|GetSpawnPoint)
    (:Is%20Valid
      (return (Transformation|GetActorTransform (LocalVariables|GetSpawnPoint))))
    (:Is%20Not%20Valid
      (Development|PrintString "No Available Spawn Points Found Spawn At 000" true true "(R=0.000000,G=0.660000,B=1.000000,A=1.000000)" 1e+01)
      (return (Math|Transform|MakeTransform "0, 0, 0" "0, 0, 0" "1.000000,1.000000,1.000000")))))